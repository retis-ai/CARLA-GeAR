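; Ambulance Blueprint that applies an image file to its decal at runtime.
; On BeginPlay, after the parent's logic, it sets the patch decal material and creates a dynamic instance of it.
; It imports the texture from a file path and feeds it to the instance's texture parameter, hiding the decal in game if the import fails.
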(event `self.ReceiveBeginPlay`
  (bind _decal (`self.Decal`))
  (`parent.ReceiveBeginPlay`)
  (`DecalComponent.SetDecalMaterial` _decal "/Game/Carla/Mat_patch.Mat_patch")
  (bind _returnvalue (`DecalComponent.CreateDynamicMaterialInstance` _decal))
  (bind _output_get (set `self.DynamicMat_auto` _returnvalue))
  (bind _returnvalue_2 (`KismetRenderingLibrary.ImportFileAsTexture2D` (`self.filepath_auto`)))
  (if (`KismetSystemLibrary.IsValid` _returnvalue_2)
    (`MaterialInstanceDynamic.SetTextureParameterValue` _output_get "TextureParam" _returnvalue_2)
    (else
      (`SceneComponent.SetHiddenInGame` _decal true false))))

(fn `UserConstructionScript`
  (`parent.UserConstructionScript`))