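; BP_Decal_Billboard_Auto is a decal actor that displays an image loaded from a file at runtime.
; On BeginPlay it applies Mat_patch to its Decal component, creates a dynamic material instance and passes both to LoadPatch.
; LoadPatch imports FilepathAuto as a Texture2D and assigns it to TextureParam, or hides the decal in game if the import fails.
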(event `self.ReceiveBeginPlay`
  (bind _decal (`self.Decal`))
  (`DecalComponent.SetDecalMaterial` _decal "/Game/Carla/Mat_patch.Mat_patch")
  (bind _returnvalue (`DecalComponent.CreateDynamicMaterialInstance` _decal))
  (bind _output_get (set `self.DynamicMat_auto` _returnvalue))
  (`self.Load Patch` _decal _output_get))

(fn `Load Patch`
  (params (Decal :type "DecalComponent Object Reference") (DynMat :type "MaterialInstanceDynamic Object Reference"))
  (bind _returnvalue (`KismetRenderingLibrary.ImportFileAsTexture2D` (`self.filepath_auto`)))
  (if (`KismetSystemLibrary.IsValid` _returnvalue)
    (`MaterialInstanceDynamic.SetTextureParameterValue` DynMat "TextureParam" _returnvalue)
    (else
      (`SceneComponent.SetHiddenInGame` Decal true false)))
  (return))

(fn `UserConstructionScript`)